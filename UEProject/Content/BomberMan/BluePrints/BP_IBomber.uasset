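; BP_IBomber is a bomber pawn Blueprint for the BomberMan game, apparently a base that provides shared movement.
; MoveFrontBack and MoveRightLeft push BomberMesh with physics forces along world X and Y, scaled by the input axis value.
; The OnSteroids power-up flag doubles that force.
; DropBomb and Event_GotFlamed are empty stubs, and the file has no active BeginPlay or Tick logic.
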(event Custom|Event_GotFlamed)

(event EventBeginPlay)

(event EventTick
  (params (DeltaSeconds :type Float%20%28single-precision%29)))

(fn ConstructionScript)

(fn DropBomb
  (params (PlayerTransform :type Transform)))

(fn MoveFrontBack
  (params (AxisValue :type Float%20%28single-precision%29))
  (if (Variables|Default|GetOnSteroids)
    ;[1 1 1] If On steroids(power up) -  Double speed
    (Physics|AddForce (Variables|Default|GetBomberMesh) (Math|Vector|MakeVector (* AxisValue 1e+05) 0.0 0.0) "None" false)
    (else
      ;[1 1 1] Normal speed
      (Physics|AddForce (Variables|Default|GetBomberMesh) (Math|Vector|MakeVector (* AxisValue 5e+04) 0.0 0.0) "None" false))))

(fn MoveRightLeft
  (params (AxisValue :type Float%20%28single-precision%29))
  (if (Variables|Default|GetOnSteroids) ; OnSteroids ? (AxisValue *2) : AxisValue
    ;[0.8157 1 0.8688] If On steroids(power up) -  Double speed
    (Physics|AddForce (Variables|Default|GetBomberMesh) (Math|Vector|MakeVector 0.0 (* AxisValue 1e+05) 0.0) "None" false)
    (else
      ;[1 1 1] Normal speed
      (Physics|AddForce (Variables|Default|GetBomberMesh) (Math|Vector|MakeVector 0.0 (* AxisValue 5e+04) 0.0) "None" false))))