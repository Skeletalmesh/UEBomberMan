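; BP_Bomb is a timed Bomberman bomb that explodes in a cross to break walls and credit its owner.
; BeginPlay activates fuse audio, waits, fires particles, then calls SeekAndDestroy along both horizontal axes.
; Each multi-object line trace flames breakable walls and increments the owner's BricksDestroyed.
; The bomb destroys itself upon any hit or after a short delay; the fixed-wall ignore lookup never executes.
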(event EventBeginPlay
  (bind _returnvalue (Transformation|GetActorRotation))
  (bind _returnvalue_2 (Transformation|GetActorLocation))
  (bind _returnvalue_3 (Math|Vector|GetForwardVector _returnvalue))
  (bind _returnvalue_4 (Math|Vector|GetRightVector _returnvalue))
  (Components|Activation|Activate (Variables|Default|GetAudioFuse) false)
  (Utilities|FlowControl|Delay 4.0)
  (Components|Activation|Activate (Variables|Default|GetP_BombXY) true)
  (CallFunction|SeekandDestroy _returnvalue_2 _returnvalue_3 1.0)
  (CallFunction|SeekandDestroy _returnvalue_2 _returnvalue_3 -1.0)
  (CallFunction|SeekandDestroy _returnvalue_2 _returnvalue_4 1.0)
  (CallFunction|SeekandDestroy _returnvalue_2 _returnvalue_4 -1.0)
  (Utilities|FlowControl|Delay 1.0)
  (Actor|DestroyActor))

(event Collision|EventActorBeginOverlap
  (params (OtherActor :type Actor%20Object%20Reference)))

(event EventTick
  (params (DeltaSeconds :type Float%20%28single-precision%29)))

(fn ConstructionScript)

(fn SeekandDestroy
  (params (TraceLocation :type Vector%20%28by%20ref%29) (AxisVector :type Vector%20%28by%20ref%29) (Direction :type Float%20%28single-precision%29))
  (bind _ownerbomber (Variables|Default|GetOwnerBomber))
  (bind (_outhits _returnvalue) (Class|KismetSystemLibrary|LineTraceMultiforObjects TraceLocation (+ TraceLocation (* (* AxisVector Direction) (Variables|Default|GetTraceDistance))) (Utilities|Array|MakeArray "ObjectTypeQuery2" "ObjectTypeQuery3" "ObjectTypeQuery6") false (stale _outactors) "None" true))
  (if _returnvalue
    (for _array_element _outhits
      (bind _asbp_breakable_wall (Utilities|Casting|CastToBP_BreakableWall (.HitActor (Collision|BreakHitResult _array_element))))
      (Default|GotFlamed _asbp_breakable_wall)
      (bind _result (Math|Integer|IncrementInt (Variables|/Game/BomberMan/BluePrints/BP_IBomber.BP_IBomber_C|GetBricksDestroyed _ownerbomber))
        (:%20%20
          (Variables|/Game/BomberMan/BluePrints/BP_IBomber.BP_IBomber_C|SetBricksDestroyed _ownerbomber _result))))
    (Actor|DestroyActor)))