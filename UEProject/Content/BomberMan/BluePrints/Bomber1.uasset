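; Bomber1 is the Player 1 Blueprint in a two-player BomberMan game, and it also relays Player 2's input.
; Forward1 and Right1 axis events push its Player component along X and Y with scaled physics forces.
; Forward2 and Right2 look up Bomber2 actors with GetAllActorsOfClass on each axis event and pass the values through interface calls To2P and Right2p.
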(event EventBeginPlay)

(event Collision|EventActorBeginOverlap
  (params (OtherActor :type Actor%20Object%20Reference)))

(event EventTick
  (params (DeltaSeconds :type Float%20%28single-precision%29)))

(event Input|AxisEvents|InputAxisForward1
  (params (AxisValue :type Float%20%28single-precision%29))
  ;[1 1 1] Forward Player 1
  (Physics|AddForce (Variables|Default|GetPlayer) (Math|Vector|MakeVector (* AxisValue 3e+05) 0.0 0.0) "None" false))

(event Input|AxisEvents|InputAxisRight1
  (params (AxisValue :type Float%20%28single-precision%29))
  ;[1 1 1] Right Player1
  (Physics|AddForce (Variables|Default|GetPlayer) (Math|Vector|MakeVector 0.0 (* AxisValue 3e+05) 0.0) "None" false))

(event Input|AxisEvents|InputAxisRight2
  (params (AxisValue :type Float%20%28single-precision%29))
  ;[1 1 1] Send Right2 inputs to player2
  (bind _outactors (Actor|GetAllActorsOfClass "/Game/BomberMan/BluePrints/Bomber2.Bomber2_C"))
  (Default|Right2p _outactors AxisValue))

(event Input|AxisEvents|InputAxisForward2
  (params (AxisValue :type Float%20%28single-precision%29))
  ;[1 1 1] Send Forward2 inputs to player2 via Interface
  (bind _outactors (Actor|GetAllActorsOfClass "/Game/BomberMan/BluePrints/Bomber2.Bomber2_C"))
  (Default|To2P _outactors AxisValue))

(fn ConstructionScript)